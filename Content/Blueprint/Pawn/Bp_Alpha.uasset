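; Player pawn that dodges across a grid of lanes in Y and Z and is destroyed when HitObstacle is called.
; Initialize takes lane counts and size from the level manager and starts the pawn in a middle lane.
; Directional inputs and touch swipes, detected on Tick past a threshold, share the same move logic.
; Each bounded move plays a roll or dash montage and timeline-lerps the location, with BeMoving blocking overlapping moves.
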(event `self.ReceiveBeginPlay`
  (`self.Initialize`))

(event `InputAction|Left`
  (params (Key :type "Key Structure"))
  (bind (_returnvalue_x _returnvalue_y) (`KismetMathLibrary.BreakVector` (`self.K2_GetActorLocation`)))
  (bind (_returnvalue_x_2 _returnvalue_y_2 _returnvalue_z) (`KismetMathLibrary.BreakVector` (`self.K2_GetActorLocation`)))
  (:`Pressed`
    ;[1 1 1] PRessed left while in the left most lane
    (if (<= (`self.CurrentLaneY`) 1) :!label _label
      _
      (elif (not (`self.Be moving`))
        (set `self.Be moving` true)
        (if (not (`self.Is rolling Left`))
          (`|PlayMontage` (`self.Alpha_Pawn`) "/Game/Assets/Alpha/Animations/Alpha_RollLeft.Alpha_RollLeft"
            (:`then`
              (set `self.Target Position Y` (- _returnvalue_y (`self.LaneWidth`)))
              (bind (_direction _move) (`Timeline|Timeline_2` :!via `PlayFromStart`)
                (:`Update`
                  (`self.K2_SetActorLocation` (`KismetMathLibrary.MakeVector` _returnvalue_x_2 (`KismetMathLibrary.Lerp` _returnvalue_y_2 (`self.Target Position Y`) _move) _returnvalue_z)))
                (:`Finished`
                  (set `self.Be moving` false)
                  (`/Engine/EditorBlueprintResources/StandardMacros.DecrementInt` (`self.CurrentLaneY`)))))))))))

(event `self.ReceiveTick`
  (params (DeltaSeconds :type "Float (single-precision)"))
  (bind (_returnvalue_x _returnvalue_y _returnvalue_z) (`KismetMathLibrary.BreakVector` (`self.K2_GetActorLocation`)))
  (bind (_returnvalue_x_2 _returnvalue_y_2 _returnvalue_z_2) (`KismetMathLibrary.BreakVector` (`self.K2_GetActorLocation`)))
  (bind (_returnvalue_x_3 _returnvalue_y_3) (`KismetMathLibrary.BreakVector` (`self.K2_GetActorLocation`)))
  (bind (_returnvalue_x_4 _returnvalue_y_4 _returnvalue_z_3) (`KismetMathLibrary.BreakVector` (`self.K2_GetActorLocation`)))
  (bind (_returnvalue_x_5 _returnvalue_y_5 _returnvalue_z_4) (`KismetMathLibrary.BreakVector` (`self.K2_GetActorLocation`)))
  (bind (_returnvalue_x_6 _returnvalue_y_6 _returnvalue_z_5) (`KismetMathLibrary.BreakVector` (`self.K2_GetActorLocation`)))
  (bind (_locationx _locationy) (`PlayerController.GetInputTouchState` (`GameplayStatics.GetPlayerController` 0) "Touch1"))
  (bind _returnvalue (`KismetMathLibrary.MakeVector2D` _locationx _locationy))
  (bind (_x _y) (`KismetMathLibrary.BreakVector2D` (- (`self.StartLoc`) (`self.EndLoc`))))
  ;[1 1 1] Swipe
  (if (`self.Is pressed`)
    (if (>= (`KismetMathLibrary.VSize2D` (- (`self.StartLoc`) _returnvalue)) (`self.Threshold`))
      (`/Engine/EditorBlueprintResources/StandardMacros.DoOnce` false :!label _label_2
        (:`Completed`
          (set `self.EndLoc` _returnvalue)
          (if (> (`KismetMathLibrary.Abs` _x) (`KismetMathLibrary.Abs` _y))
            (if (> _x 0.0)
              (`KismetSystemLibrary.PrintString` "Left" false)
              (goto _label)
              (else
                (`KismetSystemLibrary.PrintString` "Right" false)
                ;[1 1 1] Pressed Right While in right most lane
                (if (== (`self.CurrentLaneY`) (`/Game/Blueprint/LevelManager/Bp_LevelManager.Number of lanes Y` (`self.LevelManagerRef`))) :!label _label_3
                  _
                  (elif (not (`self.Be moving`))
                    (set `self.Be moving` true)
                    (if (not (`self.Is rolling Right`))
                      (`|PlayMontage` (`self.Alpha_Pawn`) "/Game/Assets/Alpha/Animations/Alpha_RollRight.Alpha_RollRight"
                        (:`OnBlendOut`
                          (set `self.Target Position Y` (+ _returnvalue_y_3 (`self.LaneWidth`)))
                          (bind (_direction _move) (`Timeline|Timeline_0` :!via `PlayFromStart`)
                            (:`Update`
                              (`self.K2_SetActorLocation` (`KismetMathLibrary.MakeVector` _returnvalue_x_4 (`KismetMathLibrary.Lerp` _returnvalue_y_4 (`self.Target Position Y`) _move) _returnvalue_z_3)))
                            (:`Finished`
                              (set `self.Be moving` false)
                              (`/Engine/EditorBlueprintResources/StandardMacros.IncrementInt` (`self.CurrentLaneY`)))))))))))
            (elif (> _y 0.0)
              (`KismetSystemLibrary.PrintString` "up" false)
              ;[1 1 1] Pressed Up While in Up most lane
              (if (== (`self.CurrentLaneZ`) (`/Game/Blueprint/LevelManager/Bp_LevelManager.Number of lanes Z` (`self.LevelManagerRef`))) :!label _label_4
                _
                (elif (not (`self.Be moving`))
                  (set `self.Be moving` true)
                  (if (not (`self.Is DashingDown`))
                    (`|PlayMontage` (`self.Alpha_Pawn`) "/Game/Assets/Alpha/Animations/Alpha_DashArrière.Alpha_DashArrière"
                      (:`then`
                        (set `self.Target Position Z` (+ _returnvalue_z_4 (`self.LaneWidth`)))
                        (bind (_direction_2 _move_2) (`Timeline|Timeline_1` :!via `PlayFromStart`)
                          (:`Update`
                            (`self.K2_SetActorLocation` (`KismetMathLibrary.MakeVector` _returnvalue_x_6 _returnvalue_y_6 (`KismetMathLibrary.Lerp` _returnvalue_z_5 (`self.Target Position Z`) _move_2))))
                          (:`Finished`
                            (set `self.Be moving` false)
                            (`/Engine/EditorBlueprintResources/StandardMacros.IncrementInt` (`self.CurrentLaneZ`)))))))))
              (else
                (`KismetSystemLibrary.PrintString` "Down" false)
                ;[1 1 1] PRessed Down while in the Down most lane
                (if (<= (`self.CurrentLaneZ`) 1) :!label _label_5
                  _
                  (elif (not (`self.Be moving`))
                    (set `self.Be moving` true)
                    (if (not (`self.Is DashingUp`))
                      (`|PlayMontage` (`self.Alpha_Pawn`) "/Game/Assets/Alpha/Animations/Alpha_DashAvant.Alpha_DashAvant"
                        (:`then`
                          (set `self.Target Position Z` (- _returnvalue_z (`self.LaneWidth`)))
                          (bind (_direction_3 _move_3) (`Timeline|Transition` :!via `PlayFromStart`)
                            (:`Update`
                              (`self.K2_SetActorLocation` (`KismetMathLibrary.MakeVector` _returnvalue_x_2 _returnvalue_y_2 (`KismetMathLibrary.Lerp` _returnvalue_z_2 (`self.Target Position Z`) _move_3))))
                            (:`Finished`
                              (set `self.Be moving` false)
                              (`/Engine/EditorBlueprintResources/StandardMacros.DecrementInt` (`self.CurrentLaneZ`)))))))))))))))))

(event `InputAction|Right`
  (params (Key :type "Key Structure"))
  (:`Pressed`
    (goto _label_3)))

(event `InputAction|Finger`
  (params (Key :type "Key Structure"))
  (bind (_locationx _locationy) (`PlayerController.GetInputTouchState` (`GameplayStatics.GetPlayerController` 0) "Touch1"))
  ;[1 1 1] Swipe
  (:`Pressed`
    (set `self.Is pressed` true)
    (set `self.StartLoc` (`KismetMathLibrary.MakeVector2D` _locationx _locationy)))
  (:`Released`
    (set `self.Is pressed` false)
    (goto _label_2 :!via `Reset`)))

(event `InputAction|Down`
  (params (Key :type "Key Structure"))
  (:`Pressed`
    (goto _label_5)))

(event `InputAction|Up`
  (params (Key :type "Key Structure"))
  (:`Pressed`
    (goto _label_4)))

(fn `HitObstacle`
  (`self.K2_DestroyActor`))

(fn `Initialize`
  (bind (_levelmanager _levelmanagerfound) (`/Game/Blueprint/Librairy/BPF_lib.GetLevelManager`))
  (if _levelmanagerfound
    (set `self.LevelManagerRef` _levelmanager)
    (set `self.CurrentLaneY` (+ (/ (`/Game/Blueprint/LevelManager/Bp_LevelManager.Number of lanes Y` (`self.LevelManagerRef`)) 2) 1))
    (set `self.CurrentLaneZ` (+ (/ (`/Game/Blueprint/LevelManager/Bp_LevelManager.Number of lanes Z` (`self.LevelManagerRef`)) 2) 1))
    (set `self.LaneWidth` (`/Game/Blueprint/LevelManager/Bp_LevelManager.LaneSize` (`self.LevelManagerRef`)))
    (else
      (`KismetSystemLibrary.PrintString` "NoLEvelManager "))))

(fn `Is DashingDown`
  (returns (ReturnValue :type Boolean))
  (return (`AnimInstance.Montage_IsPlaying` (`SkeletalMeshComponent.GetAnimInstance` (`self.Alpha_Pawn`)) "/Game/Assets/Alpha/Animations/Alpha_DashArrière.Alpha_DashArrière")))

(fn `Is DashingUp`
  (returns (ReturnValue :type Boolean))
  (return (`AnimInstance.Montage_IsPlaying` (`SkeletalMeshComponent.GetAnimInstance` (`self.Alpha_Pawn`)) "/Game/Assets/Alpha/Animations/Alpha_DashAvant.Alpha_DashAvant")))

(fn `Is rolling Left`
  (returns (ReturnValue :type Boolean))
  (return (`AnimInstance.Montage_IsPlaying` (`SkeletalMeshComponent.GetAnimInstance` (`self.Alpha_Pawn`)) "/Game/Assets/Alpha/Animations/Alpha_RollLeft.Alpha_RollLeft")))

(fn `Is rolling Right`
  (returns (ReturnValue :type Boolean))
  (return (`AnimInstance.Montage_IsPlaying` (`SkeletalMeshComponent.GetAnimInstance` (`self.Alpha_Pawn`)) "/Game/Assets/Alpha/Animations/Alpha_RollRight.Alpha_RollRight")))

(fn `UserConstructionScript`)