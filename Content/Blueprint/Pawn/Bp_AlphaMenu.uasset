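; Menu pawn for the Alpha character that plays idle montages on its skeletal mesh when the level is "Menu".
; Tick checks the level name and drives a latent chain of Delays and montages: nod (Hochement), leg idle, then scratch (Gratter).
; Tick re-enters the first Delay whenever it finishes, so the sequence repeats without an explicit loop.
; The scratch delay follows the leg montage's start, not its completion.
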(event `self.ReceiveBeginPlay`)

(event `self.ReceiveTick`
  (params (DeltaSeconds :type "Float (single-precision)"))
  (bind _returnvalue (`GameplayStatics.GetCurrentLevelName` true))
  (if (`KismetStringLibrary.EqualEqual_StrStr` _returnvalue "Menu")
    (`KismetSystemLibrary.Delay` 15.0)
    (`|PlayMontage` (`self.Alpha`) "/Game/Assets/Alpha/Animations/Alpha_Hochement.Alpha_Hochement"
      (:`OnCompleted`
        (`KismetSystemLibrary.Delay` 10.0)
        (`|PlayMontage` (`self.Alpha`) "/Game/Assets/Alpha/Animations/Alpha_IddleJambes.Alpha_IddleJambes"
          (:`then`
            (`KismetSystemLibrary.Delay` 10.0)
            (`|PlayMontage` (`self.Alpha`) "/Game/Assets/Alpha/Animations/Alpha_Gratter.Alpha_Gratter"
              (:`OnCompleted`
                (`KismetSystemLibrary.Delay` 10.0)))))))))

(fn `UserConstructionScript`)