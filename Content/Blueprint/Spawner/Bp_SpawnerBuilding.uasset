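; Building spawner that lays out a continuous row of tiles along X and recycles them as they go out of bounds.
; On BeginPlay it spawns the tiles through the parent's SpawnActor, measures width from the first one's bounds and places each behind the last along +X.
; When a tile hits the bounds, it is teleported one width past RearTile after a tiny delay and becomes the new RearTile.
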(event `self.ReceiveBeginPlay`
  (bind (_returnvalue_x _returnvalue_y) (`KismetMathLibrary.BreakVector` (`self.K2_GetActorLocation` (`self.RearTile`))))
  (`parent.ReceiveBeginPlay`)
  (for _index (range (+ (`self.ActorsRequiredCount`) 1))
    (if (== _index 0)
      (bind _returnvalue (`self.SpawnActor` (`self.SpawnActorType`)))
      (set `self.RearTile` _returnvalue)
      (set `self.TileSize` (* (.x (`.BoxExtent` (`self.GetActorBounds` _returnvalue false false))) 2.0))
      (`self.K2_SetActorLocation` (`self.RearTile`) (`self.K2_GetActorLocation`) false false)
      (else
        (bind _returnvalue_2 (`self.SpawnActor` (`self.SpawnActorType`)))
        (`self.K2_SetActorLocation` _returnvalue_2 (`KismetMathLibrary.MakeVector` (+ _returnvalue_x (`self.TileSize`)) _returnvalue_y) false false)
        (set `self.RearTile` _returnvalue_2)))))

(event `self.SpawnedActorHitBounds`
  (params (`Out of Bounds` :type "Actor Object Reference"))
  (bind (_returnvalue_x _returnvalue_y _returnvalue_z) (`KismetMathLibrary.BreakVector` (`self.K2_GetActorLocation` (`self.RearTile`))))
  (`KismetSystemLibrary.Delay` 0.001)
  (`self.K2_SetActorLocation` `Out of Bounds` (`KismetMathLibrary.MakeVector` (+ _returnvalue_x (`self.TileSize`)) _returnvalue_y _returnvalue_z) false true)
  (set `self.RearTile` `Out of Bounds`))

(fn `SpawnActor`
  (params (SpawnActorType :type "Actor Class Reference"))
  (returns (ReturnValue :type "Actor Object Reference"))
  (bind _returnvalue (`parent.SpawnActor` SpawnActorType))
  (return _returnvalue))

(fn `UserConstructionScript`
  (`parent.UserConstructionScript`))