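; Obstacle spawner that repeatedly places waves of obstacles across a lane grid while the level is playing.
; The level manager supplies obstacle classes, footprints, grid size and required path count; a delay separates waves.
; PlaceObstacle picks random types and lanes, marking a boolean occupancy array until the path limit is reached, staggering spawns along X.
; Only 1x1 and 3x1 footprints are handled; 3x1 is flagged as able to block every path.
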(event `self.ReceiveBeginPlay`
  (bind (_levelmanager _levelmanagerfound) (`/Game/Blueprint/Librairy/BPF_lib.GetLevelManager`))
  (if _levelmanagerfound
    (set `self.Level Manager Ref` _levelmanager)
    (`self.Line Up Next Obstacle Spawn`)))

(event `Line Up Next Obstacle Spawn`
  (bind _level_manager_ref (`self.Level Manager Ref`))
  (bind _level_manager_ref_2 (`self.Level Manager Ref`))
  (if (`/Game/Blueprint/LevelManager/Bp_LevelManager.IsPlaying` _level_manager_ref_2) :!label _label
    (`self.Place Obstacle` (* (`KismetMathLibrary.Conv_IntToDouble` (`/Game/Blueprint/LevelManager/Bp_LevelManager.GapBetweenObstacle` _level_manager_ref_2)) 0.75))
    (`KismetSystemLibrary.Delay` (/ (`KismetMathLibrary.Conv_IntToDouble` (`/Game/Blueprint/LevelManager/Bp_LevelManager.GapBetweenObstacle` _level_manager_ref)) (`KismetMathLibrary.Abs` (`/Game/Blueprint/LevelManager/Bp_LevelManager.LevelSpeed` _level_manager_ref))))
    (goto _label)))

(fn `ConvertLineNumberToCoordinate`
  (params (`Line Number` :type Integer))
  (returns (`Line Y` :type Integer) (`Column Z` :type Integer))
  (bind _level_manager_ref (`self.Level Manager Ref`))
  (return (/ `Line Number` (`/Game/Blueprint/LevelManager/Bp_LevelManager.Number of lanes Y` _level_manager_ref)) (mod `Line Number` (`/Game/Blueprint/LevelManager/Bp_LevelManager.Number of lanes Z` _level_manager_ref))))

(fn `GetRamdomLane`
  (returns (ReturnValue :type Integer))
  (return (`KismetMathLibrary.RandomIntegerInRange` 0 (- (`self.NumberOfLane`) 1))))

(fn `Place Obstacle`
  (params (SizeOfSpawnZone :type "Float (double-precision)"))
  (locals (NbOfObstacleToCreate :type Integer) (ObstacleAlreadySpawn :type Integer) (ObstacleToCreate :type "Array of Boolean") (NewObstacleChoise :type Boolean) (LineOfNewObstacle :type Integer :default 0) (IndexOfNewObstacleClass :type Integer))
  (bind (_line_y _column_z) (`self.ConvertLineNumberToCoordinate` (`local.LineOfNewObstacle`)))
  (bind _returnvalue (`KismetMathLibrary.FTrunc` (* (`self.ConvertLineNumberToCoordinate` (`local.LineOfNewObstacle`)) (`KismetMathLibrary.Conv_IntToDouble` (`/Game/Blueprint/LevelManager/Bp_LevelManager.Number of lanes Z` (`self.Level Manager Ref`))))))
  (for _ (range (`self.NumberOfLane`))
    (`KismetArrayLibrary.Array_Add` (`local.ObstacleToCreate`)))
  (while (> (- (`self.NumberOfLane`) (`local.NbOfObstacleToCreate`)) (`/Game/Blueprint/LevelManager/Bp_LevelManager.NumberOfPath` (`self.Level Manager Ref`)))
    (set `local.NewObstacleChoise` false)
    (while (not (`local.NewObstacleChoise`))
      (bind _output_get (set `local.IndexOfNewObstacleClass` (`KismetMathLibrary.RandomIntegerInRange` 0 (- (`KismetArrayLibrary.Array_Length` (`/Game/Blueprint/LevelManager/Bp_LevelManager.ObstacleTypeListe` (`self.Level Manager Ref`))) 1))))
      (bind (_output_x _output_y) (`KismetMathLibrary.BreakVector2D` (`|GetArrayItem` (`/Game/Blueprint/LevelManager/Bp_LevelManager.ObstacleTypeSizeListe` (`self.Level Manager Ref`)) _output_get)))
      (switch `int` (`KismetMathLibrary.FTrunc` _output_x)
        (:`1`
          (bind _returnvalue_2 (`KismetMathLibrary.FTrunc` _output_y))
          (switch `int` _returnvalue_2
            (:`1`
              (bind _output_get_2 (set `local.LineOfNewObstacle` (`self.GetRamdomLane`)))
              (if (not (`|GetArrayItem` (`local.ObstacleToCreate`) _output_get_2))
                (`KismetArrayLibrary.Array_Set` (`local.ObstacleToCreate`) (`local.LineOfNewObstacle`) true)
                (`/Engine/EditorBlueprintResources/StandardMacros.IncrementInt` (`local.NbOfObstacleToCreate`)
                  (:`  `
                    (set `local.NewObstacleChoise` true)))))))
        (:`2`
          (switch `int` _returnvalue_2))
        (:`3`
          (switch `int` _returnvalue_2
            (:`1`
              ;[1 1 1] Peut bloquer tout les chemin a corriger
              (bind _output_get_3 (set `local.LineOfNewObstacle` (`self.GetRamdomLane`)))
              (if (not (`|GetArrayItem` (`local.ObstacleToCreate`) _output_get_3))
                (for _index (range (+ _returnvalue 1))
                  (`KismetArrayLibrary.Array_Set` (`local.ObstacleToCreate`) (+ _index _returnvalue) true)
                  (bind _output_get_4 (set `local.NbOfObstacleToCreate` (+ (stale _output_get_4) (`/Game/Blueprint/LevelManager/Bp_LevelManager.Number of lanes Z` (`self.Level Manager Ref`)))))
                  (set `local.NewObstacleChoise` true))))))))
    (bind _returnvalue_3 (`self.SpawnActor` (`|GetArrayItem` (`/Game/Blueprint/LevelManager/Bp_LevelManager.ObstacleTypeListe` (`self.Level Manager Ref`)) (`local.IndexOfNewObstacleClass`))))
    (bind _asbp_lv1_obstacle (cast `/Game/Blueprint/Obstacles/BP_LV1_Obstacle` _returnvalue_3))
    (`/Game/Blueprint/Obstacles/BP_LV1_Obstacle.Place New` _asbp_lv1_obstacle self (* (`local.ObstacleAlreadySpawn`) (/ SizeOfSpawnZone (`KismetMathLibrary.Conv_IntToDouble` (`local.NbOfObstacleToCreate`)))) _line_y _column_z)
    (`/Engine/EditorBlueprintResources/StandardMacros.IncrementInt` (`local.ObstacleAlreadySpawn`))))

(fn `SpawnActor`
  (params (SpawnActorType :type "Actor Class Reference"))
  (returns (ReturnValue :type "Actor Object Reference"))
  (bind _returnvalue (`parent.SpawnActor` SpawnActorType))
  (return _returnvalue))

(fn `SpawnedActorHitBounds`
  (params (`Out of Bounds` :type "Actor Object Reference"))
  (`parent.SpawnedActorHitBounds` null)
  (`self.K2_DestroyActor` `Out of Bounds`))

(fn `UserConstructionScript`
  (`parent.UserConstructionScript`))