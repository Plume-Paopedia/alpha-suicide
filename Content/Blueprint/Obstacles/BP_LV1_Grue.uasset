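; Level 1 crane ("Grue") obstacle that positions itself relative to a spawner on the lane grid.
; Place New offsets X by the given value and Z by column times the level manager's LaneSize.
; The line value picks one of two asymmetric lane-scaled Y offsets, rotating the crane 180 degrees when below 1.
; The final move is swept, and the event graph holds no active logic.
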(fn `Place New`
  (params (Spawner :type "/Game/Blueprint/Spawner/Bp_SpawnerObstacle Object Reference") (RelativeX :type "Float (double-precision)") (LineY :type Integer) (ColumnZ :type Integer))
  (locals (ShiftY :type Integer))
  (bind (_returnvalue_x _returnvalue_y _returnvalue_z) (`KismetMathLibrary.BreakVector` (`self.K2_GetActorLocation` Spawner)))
  (bind _lanesize (`/Game/Blueprint/LevelManager/Bp_LevelManager.LaneSize` (`/Game/Blueprint/Librairy/BPF_lib.GetLevelManager`)))
  (if (>= LineY 1)
    (set `local.ShiftY` (`KismetMathLibrary.FTrunc` (* -2 _lanesize)))
    (else
      (bind _output_get (set `local.ShiftY` (`KismetMathLibrary.FTrunc` (* 4 _lanesize))))
      (`self.K2_SetActorRelativeRotation` (struct :`Roll` 180.0))))
  (`self.K2_SetActorLocation` (`KismetMathLibrary.MakeVector` (+ RelativeX _returnvalue_x) (+ (`KismetMathLibrary.Conv_IntToDouble` _output_get) _returnvalue_y) (+ (* ColumnZ (`/Game/Blueprint/LevelManager/Bp_LevelManager.LaneSize` (`self.LevelManagerRef`))) _returnvalue_z)) true))

(fn `UserConstructionScript`
  (`parent.UserConstructionScript`))