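; BP_LV1_Obstacle is a level 1 obstacle that ends the game when Bp_Alpha overlaps its static mesh.
; On overlap it calls HitObstacle on Bp_Alpha, then GameOver on the level manager, printing a warning if none is found.
; PlaceNew positions it on a lane grid relative to a spawner using the manager's LaneSize.
; It also stores a parent reference; random Y-scaling logic is present but disconnected.
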(event `self.ReceiveBeginPlay`
  (bind (_levelmanager _levelmanagerfound) (`/Game/Blueprint/Librairy/BPF_lib.GetLevelManager`))
  (if _levelmanagerfound
    (set `self.LevelManagerRef` _levelmanager)))

(event `self.StaticMesh.OnComponentBeginOverlap`
  (params (OverlappedComponent :type "PrimitiveComponent Object Reference") (OtherActor :type "Actor Object Reference") (OtherComp :type "PrimitiveComponent Object Reference") (OtherBodyIndex :type Integer) (bFromSweep :type Boolean) (SweepResult :type "HitResult Structure (by ref)"))
  (bind (_levelmanager _levelmanagerfound) (`/Game/Blueprint/Librairy/BPF_lib.GetLevelManager`))
  (bind _asbp_alpha (cast `/Game/Blueprint/Pawn/Bp_Alpha` OtherActor))
  (`/Game/Blueprint/Pawn/Bp_Alpha.HitObstacle` _asbp_alpha)
  (if _levelmanagerfound
    (`/Game/Blueprint/LevelManager/Bp_LevelManager.GameOver` _levelmanager)
    (else
      (`KismetSystemLibrary.PrintString` "No level manager"))))

(fn `Place New`
  (params (Spawner :type "/Game/Blueprint/Spawner/Bp_SpawnerObstacle Object Reference") (RelativeX :type "Float (double-precision)") (LineY :type Integer) (ColumnZ :type Integer))
  (bind (_returnvalue_x _returnvalue_y _returnvalue_z) (`KismetMathLibrary.BreakVector` (`self.K2_GetActorLocation` Spawner)))
  (bind _lanesize (`/Game/Blueprint/LevelManager/Bp_LevelManager.LaneSize` (`self.LevelManagerRef`)))
  (`self.K2_SetActorLocation` (`KismetMathLibrary.MakeVector` (+ RelativeX _returnvalue_x) (+ (* LineY _lanesize) _returnvalue_y) (+ (* ColumnZ _lanesize) _returnvalue_z)) true))

(fn `ReturnParent`
  (returns (Parent :type "/Game/Blueprint/Spawner/Bp_Spawner Object Reference"))
  (return (`self.Parent Ref`)))

(fn `Set Parent`
  (params (Parent :type "/Game/Blueprint/Spawner/Bp_Spawner Object Reference"))
  (returns (Return :type Boolean))
  (set `self.Parent Ref` Parent)
  (return false))

(fn `UserConstructionScript`)