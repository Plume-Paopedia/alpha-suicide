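; Level manager Blueprint that tracks obstacle type sizes, out-of-bounds detection and the playing state.
; On BeginPlay it briefly spawns each listed obstacle class to cache its width and height, then destroys it.
; The construction script sizes and places the LevelBounds box, whose overlaps notify the entering actor's parent through SpawnedActorHitBounds.
; GameOver clears the IsPlaying flag.
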(event `self.ReceiveBeginPlay`
  (for _array_element (`self.ObstacleTypeListe`)
    (bind _returnvalue (`|SpawnActorFromClass` _array_element (`self.GetTransform`) "Undefined" "OverrideRootScale" null null))
    (`KismetArrayLibrary.Array_Add` (`self.ObstacleTypeSizeListe`) (`KismetMathLibrary.MakeVector2D` (`KismetMathLibrary.Conv_IntToDouble` (`/Game/Blueprint/Obstacles/BP_LV1_Obstacle.Width` _returnvalue)) (`KismetMathLibrary.Conv_IntToDouble` (`/Game/Blueprint/Obstacles/BP_LV1_Obstacle.Height` _returnvalue))))
    (`self.K2_DestroyActor` _returnvalue)))

(event `self.LevelBounds.OnComponentBeginOverlap`
  (params (OverlappedComponent :type "PrimitiveComponent Object Reference") (OtherActor :type "Actor Object Reference") (OtherComp :type "PrimitiveComponent Object Reference") (OtherBodyIndex :type Integer) (bFromSweep :type Boolean) (SweepResult :type "HitResult Structure (by ref)"))
  (bind _parent (message `/Game/Blueprint/Interface/BPI_Spwanable.ReturnParent` OtherActor))
  (`/Engine/EditorBlueprintResources/StandardMacros.IsValid` _parent
    (:`Is Valid`
      (`/Game/Blueprint/Spawner/Bp_Spawner.SpawnedActorHitBounds` _parent OtherActor))))

(fn `GameOver`
  (set `self.IsPlaying` false))

(fn `UserConstructionScript`
  (bind _levelbounds (`self.LevelBounds`))
  (`BoxComponent.SetBoxExtent` _levelbounds (`self.OutOfBoundBoxScale`) true)
  (`SceneComponent.K2_SetWorldLocation` _levelbounds (`self.OutOfBoundBoxLocation`) false false))